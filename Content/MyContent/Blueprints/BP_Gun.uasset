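; VR gun that is assembled by hand from stock, magazine, bolt, charging and trigger parts.
; Child grip and release events keep a HeldBy map from each gripped part to its gripping controller.
; When a held part overlaps its collision volume, that controller drops and sockets it to the static mesh and clears the entry.
; The charging handler checks and sockets CharginCollision itself, rather than a separate part component.
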(event `VRGripInterface.OnChildGrip`
  (params (GrippingController :type "GripMotionControllerComponent Object Reference") (GripInformation :type "BPActorGripInformation Structure (by ref)"))
  (bind (_gripid _griptargettype _grippedobject) (break `BPActorGripInformation` GripInformation))
  ;[1 1 1] Grab
  (`/Engine/EditorBlueprintResources/StandardMacros.IsValid` _grippedobject
    (:`Is Valid`
      (`BlueprintMapLibrary.Map_Add` (`self.heldBy`) _grippedobject GrippingController))))

(event `VRGripInterface.OnChildGripRelease`
  (params (ReleasingController :type "GripMotionControllerComponent Object Reference") (GripInformation :type "BPActorGripInformation Structure (by ref)") (bWasSocketed :type Boolean))
  (bind (_gripid _griptargettype _grippedobject) (break `BPActorGripInformation` GripInformation))
  ;[1 1 1] Let go
  (`/Engine/EditorBlueprintResources/StandardMacros.IsValid` _grippedobject
    (:`Is Valid`
      (`BlueprintMapLibrary.Map_Remove` (`self.heldBy`) _grippedobject))))

(event `self.StockCollision.OnComponentBeginOverlap`
  (params (OverlappedComponent :type "PrimitiveComponent Object Reference") (OtherActor :type "Actor Object Reference") (OtherComp :type "PrimitiveComponent Object Reference") (OtherBodyIndex :type Integer) (bFromSweep :type Boolean) (SweepResult :type "HitResult Structure (by ref)"))
  (bind _stock (`self.Stock`))
  (bind _stock_2 (`self.Stock`))
  (bind (_value _returnvalue) (`BlueprintMapLibrary.Map_Find` (`self.heldBy`) _stock_2))
  ;[1 1 1] Make Stock Collide
  (if (and _returnvalue (== _stock_2 OtherComp))
    (bind _returnvalue_2 (`GripMotionControllerComponent.DropAndSocketObject` _value (`VRExpansionFunctionLibrary.MakeTransform_NetQuantize` (0.0 0.0 0.0)) _stock 0 (`self.StaticMeshComponent`) "None" true))
    (if _returnvalue_2
      (`BlueprintMapLibrary.Map_Remove` (`self.heldBy`) _stock))))

(event `self.MagazineCollision.OnComponentBeginOverlap`
  (params (OverlappedComponent :type "PrimitiveComponent Object Reference") (OtherActor :type "Actor Object Reference") (OtherComp :type "PrimitiveComponent Object Reference") (OtherBodyIndex :type Integer) (bFromSweep :type Boolean) (SweepResult :type "HitResult Structure (by ref)"))
  (bind _magazine (`self.Magazine`))
  (bind _magazine_2 (`self.Magazine`))
  (bind (_value _returnvalue) (`BlueprintMapLibrary.Map_Find` (`self.heldBy`) _magazine))
  ;[1 1 1] Magazine Collide
  (if (and _returnvalue (== _magazine OtherComp))
    (bind _returnvalue_2 (`GripMotionControllerComponent.DropAndSocketObject` _value (`VRExpansionFunctionLibrary.MakeTransform_NetQuantize` (0.0 0.0 0.0)) _magazine_2 0 (`self.StaticMeshComponent`) "None" true))
    (if _returnvalue_2
      (`BlueprintMapLibrary.Map_Remove` (`self.heldBy`) _magazine_2))))

(event `self.BoltCollision.OnComponentBeginOverlap`
  (params (OverlappedComponent :type "PrimitiveComponent Object Reference") (OtherActor :type "Actor Object Reference") (OtherComp :type "PrimitiveComponent Object Reference") (OtherBodyIndex :type Integer) (bFromSweep :type Boolean) (SweepResult :type "HitResult Structure (by ref)"))
  (bind _bolt (`self.Bolt`))
  (bind _bolt_2 (`self.Bolt`))
  (bind (_value _returnvalue) (`BlueprintMapLibrary.Map_Find` (`self.heldBy`) _bolt))
  ;[1 1 1] Bolt collision
  (if (and _returnvalue (== _bolt OtherComp))
    (bind _returnvalue_2 (`GripMotionControllerComponent.DropAndSocketObject` _value (`VRExpansionFunctionLibrary.MakeTransform_NetQuantize` (0.0 0.0 0.0)) _bolt_2 0 (`self.StaticMeshComponent`) "None" true))
    (if _returnvalue_2
      (`BlueprintMapLibrary.Map_Remove` (`self.heldBy`) _bolt_2))))

(event `self.CharginCollision.OnComponentBeginOverlap`
  (params (OverlappedComponent :type "PrimitiveComponent Object Reference") (OtherActor :type "Actor Object Reference") (OtherComp :type "PrimitiveComponent Object Reference") (OtherBodyIndex :type Integer) (bFromSweep :type Boolean) (SweepResult :type "HitResult Structure (by ref)"))
  (bind _chargincollision (`self.CharginCollision`))
  (bind _chargincollision_2 (`self.CharginCollision`))
  (bind (_value _returnvalue) (`BlueprintMapLibrary.Map_Find` (`self.heldBy`) _chargincollision))
  ;[1 1 1] Chargin Collision
  (if (and _returnvalue (== _chargincollision OtherComp))
    (bind _returnvalue_2 (`GripMotionControllerComponent.DropAndSocketObject` _value (`VRExpansionFunctionLibrary.MakeTransform_NetQuantize` (0.0 0.0 0.0)) _chargincollision_2 0 (`self.StaticMeshComponent`) "None" true))
    (if _returnvalue_2
      (`BlueprintMapLibrary.Map_Remove` (`self.heldBy`) _chargincollision_2))))

(event `self.TriggerCollision.OnComponentBeginOverlap`
  (params (OverlappedComponent :type "PrimitiveComponent Object Reference") (OtherActor :type "Actor Object Reference") (OtherComp :type "PrimitiveComponent Object Reference") (OtherBodyIndex :type Integer) (bFromSweep :type Boolean) (SweepResult :type "HitResult Structure (by ref)"))
  (bind _trigger (`self.Trigger`))
  (bind _trigger_2 (`self.Trigger`))
  (bind (_value _returnvalue) (`BlueprintMapLibrary.Map_Find` (`self.heldBy`) _trigger))
  ;[1 1 1] Trigger Collision
  (if (and _returnvalue (== _trigger OtherComp))
    (bind _returnvalue_2 (`GripMotionControllerComponent.DropAndSocketObject` _value (`VRExpansionFunctionLibrary.MakeTransform_NetQuantize` (0.0 0.0 0.0)) _trigger_2 0 (`self.StaticMeshComponent`) "None" true))
    (if _returnvalue_2
      (`BlueprintMapLibrary.Map_Remove` (`self.heldBy`) _trigger_2))))

(fn `UserConstructionScript`)